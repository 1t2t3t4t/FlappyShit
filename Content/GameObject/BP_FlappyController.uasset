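; BP_FlappyController is the controller for a Flappy-style game, handling the HUD and score feedback.
; On BeginPlay it creates WBP_Hud, keeps a reference to it and adds it to the viewport.
; IncreasePlayerScore writes the score it receives into the HUD's ScoreText and plays a coin sound at the world origin, without storing or incrementing the value itself.
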(event EventBeginPlay
  (bind _returnvalue (UserInterface|CreateWidget "/Game/UI/WBP_Hud.WBP_Hud_C"))
  (bind _output_get (Variables|Default|SetHud _returnvalue))
  (UserInterface|Viewport|AddtoViewport _output_get 0))

(event EventTick
  (params (DeltaSeconds :type Float%20%28single-precision%29)))

(fn ConstructionScript)

(fn IncreasePlayerScore
  (params (Score :type Integer))
  (Rendering|Components|TextRender|SetText (Variables|/Game/UI/WBP_Hud.WBP_Hud_C|GetScoreText (Variables|Default|GetHud)) (Utilities|Text|ToText(String) (Utilities|String|Append "Score: " (Utilities|String|ToString(Integer) Score))))
  (Audio|PlaySoundatLocation "/Game/Sounds/SC_Coin.SC_Coin" "0, 0, 0" "0, 0, 0" 1.0 1.0 0.0 0 0 0))